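; Monster AI Blueprint, named as a special-state variant of the base monster, with an empty special-ability start event.
; SearchingRandomLocation walks the monster to random reachable points nearby, pausing briefly and re-calling itself after success or failure, then resets its counter after three moves.
; The OnPatrolWaitStart function only returns a local variable; its call to the search is disconnected, so nothing in this file starts it.
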(event Custom|Searching%20Random%20Location
  (if (< (Variables|Default|GetSearching%20Count) 3)
    (AI|AIMoveTo self (.RandomLocation (AI|Navigation|GetRandomReachablePointinRadius (Transformation|GetActorLocation) 5e+02 0 0)) 0 5.0 false
      (:OnSuccess
        _)
      (:OnFail
        _))
    (Utilities|FlowControl|Delay 1.0)
    (Math|Integer|IncrementInt (Variables|Default|GetSearching%20Count)
      (:%20%20
        (CallFunction|SearchingRandomLocation)))
    (else
      (Variables|Default|SetSearching%20Count 0))))

(event EventBeginPlay
  (|CallParentFunction))

(event Collision|EventActorBeginOverlap
  (params (OtherActor :type Actor%20Object%20Reference))
  (|CallParentFunction OtherActor) ; This node is disabled and will not be called.\nDrag off pins to build functionality.
)

(event EventTick
  (params (DeltaSeconds :type Float%20%28single-precision%29))
  (|CallParentFunction DeltaSeconds))

(event EventOnSpecialAbilityStart)

(fn ConstructionScript
  (|CallParentFunction))

(fn OnPatrolWaitStart
  (return (LocalVariables|GetNewLocalVar)))